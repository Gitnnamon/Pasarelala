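; BP_Camino is a trigger actor that lights up three lights while the first-person player character is inside its box.
; Box overlap begin casts the other actor to BP_FirstPersonCharacter and sets Luzoficial, Luzoficial1 and Luzoficial2 to a very high intensity.
; Overlap end runs the same cast and drops all three to zero intensity, switching instantly with no fade.
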(event `self.Box.OnComponentBeginOverlap`
  (params (OverlappedComponent :type "PrimitiveComponent Object Reference") (OtherActor :type "Actor Object Reference") (OtherComp :type "PrimitiveComponent Object Reference") (OtherBodyIndex :type Integer) (bFromSweep :type Boolean) (SweepResult :type "HitResult Structure (by ref)"))
  (cast `/Game/FirstPerson/Blueprints/BP_FirstPersonCharacter` OtherActor)
  (`LightComponent.SetIntensity` (`self.luzoficial`) 99900.0)
  (`LightComponent.SetIntensity` (`self.luzoficial1`) 99900.0)
  (`LightComponent.SetIntensity` (`self.luzoficial2`) 99900.0))

(event `self.Box.OnComponentEndOverlap`
  (params (OverlappedComponent :type "PrimitiveComponent Object Reference") (OtherActor :type "Actor Object Reference") (OtherComp :type "PrimitiveComponent Object Reference") (OtherBodyIndex :type Integer))
  (cast `/Game/FirstPerson/Blueprints/BP_FirstPersonCharacter` OtherActor)
  (`LightComponent.SetIntensity` (`self.luzoficial`) 0.0)
  (`LightComponent.SetIntensity` (`self.luzoficial1`) 0.0)
  (`LightComponent.SetIntensity` (`self.luzoficial2`) 0.0))

(fn `UserConstructionScript`)